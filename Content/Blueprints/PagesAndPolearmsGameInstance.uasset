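; Game instance for Pages and Polearms that manages LAN multiplayer sessions and map travel.
; Hosting creates a session and opens the Dojo landing map as a listen server, from both the immediate and success pins.
; Searching caches results and trimmed server names, which feed the PageController widget's join buttons; joining picks by index.
; Starting and ending games toggle InGame and use ServerTravel, while network and travel errors are printed.
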(event Custom|Host%20Game
  (bind _returnvalue (Game|GetPlayerController 0))
  ;[1 1 1] Hosts a game and opens the desired map
  (|Session _returnvalue 8 true
    (:then
      (Development|PrintString "Success!" :!label _label)
      (Development|ExecuteConsoleCommand "open /Game/Dojo/multiPlayerLandingArea?listen" _returnvalue)
      (Variables|Default|SetIn%20session true))
    (:OnSuccess
      (goto _label))
    (:OnFailure
      (Development|PrintString "Failed to create session"))))

(event Custom|Start%20Game
  (params (Map%20Name :type String))
  (Variables|Default|SetIn%20Game true)
  (Development|ExecuteConsoleCommand (Utilities|String|Append "ServerTravel " Map%20Name)))

(event Custom|Find%20Games
  ;[1 1 1] Gets a list of all available games, and prints off their names
  (Utilities|Array|Clear (Variables|Default|GetGames%20list))
  (Utilities|Array|Clear (Variables|Default|GetSession%20Name%20List))
  (bind _results (|FindSessions (Game|GetPlayerController 0) 8 true)
    (:OnSuccess
      (for (_array_element _array_index) _results
        (Utilities|Array|Add (Variables|Default|GetGames%20list) _array_element)
        (Utilities|Array|Add (Variables|Default|GetSession%20Name%20List) (.LeftS (Utilities|String|Split (Class|FindSessionsCallbackProxy|GetServerName _array_element) "-"))))
      (bind _aspage_controller (Utilities|Casting|CastToPageController (Game|GetPlayerController 0)))
      (Default|UpdateJoinButtons (Variables|/Game/PageController.PageController_C|GetGame%20Session%20Widget _aspage_controller) (Variables|Default|GetSession%20Name%20List)))
    (:OnFailure
      (Development|PrintString "Nothing Found"))))

(event Custom|End%20Game
  (Variables|Default|SetIn%20Game false)
  (Development|ExecuteConsoleCommand "ServerTravel multiplayerLanding "))

(event Custom|Join%20Game
  (params (Session%20number :type Integer))
  ;[1 1 1] Joins the first game listed
  (|JoinSession (Game|GetPlayerController 0) (Utilities|Array|Get(acopy) (Variables|Default|GetGames%20list) Session%20number)
    (:OnSuccess
      (Variables|Default|SetIn%20session true))
    (:OnFailure
      (Development|PrintString "Failure to join"))))

(event Custom|Destroy%20Game
  (|DestroySession (Game|GetPlayerController 0)))

(event EventHandleNetworkError
  (params (FailureType :type ENetworkFailure%20Enum :default "NetDriverAlreadyExists") (bIsServer :type Boolean))
  (Development|PrintString (Utilities|String|EnumtoString FailureType)))

(event EventHandleTravelError
  (params (FailureType :type ETravelFailure%20Enum :default "NoLevel"))
  (Development|PrintString (Utilities|String|EnumtoString FailureType)))