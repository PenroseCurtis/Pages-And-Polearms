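; Punch attack Blueprint whose Attack override only forwards the attacker and both rolls to the parent and returns its result.
; An unconnected, never-executed chain holds punch-specific resolution: random hit and damage rolls, then dodge, block and deflection checks per Page target.
; In that dead chain, dominant-hand piercing and bludgeon, scaled by deflection and reduced by hardness and padding, damage Vitality and Stamina, with results messaged through the attacker's controller.
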(fn Attack
  (params (Attacker :type Page%20Object%20Reference) (Hit%20Die%20Roll :type Float%20%28single-precision%29) (Damage%20Die%20Roll :type Float%20%28single-precision%29))
  (bind _attack_completed (|CallParentFunction Attacker Hit%20Die%20Roll Damage%20Die%20Roll))
  (return _attack_completed))