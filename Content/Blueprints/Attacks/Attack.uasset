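; Data-driven attack that resolves one action against a list of targets, with its settings loaded from a struct.
; Attack filters targets by type, range and self-targeting, checks the minimum count, then tests dodge against Dexterity and block against Guard.
; Hits deal Vitality and Stamina damage from weapon, roll and armor, scaled by deflection, and report through controller messages and attacker events.
; The critical-hit check is defined but unused by Attack.
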(fn GetValidTargets
  (params (Targets :type Array%20of%20Actor%20Object%20References) (Attacker :type Page%20Object%20Reference))
  (Utilities|Array|Clear (LocalVariables|GetLocal%20targets))
  (for _array_element Targets
    (bind _valid (CallFunction|IsTargetValid _array_element Attacker))
    (if _valid
      (Utilities|Array|Add (LocalVariables|GetLocal%20targets) _array_element)))
  (return (LocalVariables|GetLocal%20targets)))

(fn Attack
  (params (Attacker :type Page%20Object%20Reference) (Hit%20Die%20Roll :type Float%20%28single-precision%29) (Damage%20Die%20Roll :type Float%20%28single-precision%29))
  (LocalVariables|SetLocal%20Attacker Attacker)
  (LocalVariables|SetHit%20Roll Hit%20Die%20Roll)
  (LocalVariables|SetDamage%20Roll Damage%20Die%20Roll)
  (|PrintNumberofTargetsBefore)
  (bind _local_targets1 (CallFunction|GetValidTargets (Variables|Default|GetTargetList) (LocalVariables|GetLocal%20Attacker)))
  (bind _output_get (Variables|Default|SetTargetList _local_targets1))
  (|Printnumtargetsafter _output_get
    (:Out
      (bind _returnvalue (CallFunction|DoIHaveEnoughTargets))
      (if _returnvalue
        (Development|PrintString 0 "Attack!")
        (for _array_element (Variables|Default|GetTargetList)
          (bind _aspage (Utilities|Casting|CastToPage _array_element))
          (LocalVariables|SetCurrent%20Target _aspage)
          (bind _isdodged (CallFunction|IsAttackDodged? (LocalVariables|GetLocal%20Attacker) (LocalVariables|GetCurrent%20Target) true (LocalVariables|GetHit%20Roll)))
          (if _isdodged
            (bind _name (Class|WorldObject|GetName(Message) (LocalVariables|GetLocal%20Attacker)))
            (bind _name_2 (Class|WorldObject|GetName(Message) (LocalVariables|GetCurrent%20Target)))
            (Class|TurnTaking|PassMessage(Message) (Pawn|GetController (LocalVariables|GetLocal%20Attacker)) false _name (Utilities|String|Append _name " used " (Variables|Default|GetAttack%20Name) " on " _name_2 " but it was dodged") "Weapon/Default_Sword/Sword")
            (Default|EventAttackTarget Attacker (LocalVariables|GetCurrent%20Target) (Variables|Default|GetHigh/Mid/Low) (Variables|Default|GetTwoH/OneHRight/OneHLeft) "Missed")
            (else
              (bind _newparam (CallFunction|IsAttackBlocked? (LocalVariables|GetCurrent%20Target) (LocalVariables|GetLocal%20Attacker) true (LocalVariables|GetHit%20Roll)))
              (if _newparam
                (bind _name_3 (Class|WorldObject|GetName(Message) (LocalVariables|GetLocal%20Attacker)))
                (bind _name_4 (Default|GetName (LocalVariables|GetCurrent%20Target)))
                (Class|TurnTaking|PassMessage(Message) (Pawn|GetController (LocalVariables|GetLocal%20Attacker)) false _name_3 (Utilities|String|Append _name_3 " used " (Variables|Default|GetAttack%20Name) " on " _name_4 " but it was blocked") "Weapon/Default_Sword/Sword")
                (Default|EventAttackTarget Attacker (LocalVariables|GetCurrent%20Target) (Variables|Default|GetHigh/Mid/Low) (Variables|Default|GetTwoH/OneHRight/OneHLeft) "Blocked!")
                (else
                  (bind (_total_coverage1 _total_padding1 _total_hardness1) (Default|GetDefensiveStats (Variables|/Game/Characters/Page.Page_C|GetInventory (LocalVariables|GetCurrent%20Target))))
                  (bind _returnvalue_2 (CallFunction|GetDeflectionModifier (LocalVariables|GetLocal%20Attacker) (LocalVariables|GetCurrent%20Target) true (LocalVariables|GetHit%20Roll)))
                  (bind _name_5 (Class|WorldObject|GetName(Message) (LocalVariables|GetLocal%20Attacker)))
                  (bind _name_6 (Class|WorldObject|GetName(Message) (LocalVariables|GetCurrent%20Target)))
                  (Class|TurnTaking|PassMessage(Message) (Pawn|GetController Attacker) true "" (Utilities|String|Append _name_5 " used " (Variables|Default|GetAttack%20Name) " on " _name_6 " and it did " (Utilities|String|ToString(Integer) (Math|Float|Ceil (* (- (+ (Variables|Default|GetDamage) (Variables|/Game/Items/WeaponObject.WeaponObject_C|GetDamage (Variables|/Game/Items/Inventory.Inventory_C|GetDominant%20Hand (Variables|/Game/Characters/Page.Page_C|GetInventory (LocalVariables|GetLocal%20Attacker)))) (LocalVariables|GetDamage%20Roll)) (/ (+ (- _total_hardness1 (Variables|/Game/Items/WeaponObject.WeaponObject_C|GetPiercing (Variables|/Game/Items/Inventory.Inventory_C|GetDominant%20Hand (Variables|/Game/Characters/Page.Page_C|GetInventory (LocalVariables|GetLocal%20Attacker))))) (Math|Float|Absolute(Float) (- _total_hardness1 (Variables|/Game/Items/WeaponObject.WeaponObject_C|GetPiercing (Variables|/Game/Items/Inventory.Inventory_C|GetDominant%20Hand (Variables|/Game/Characters/Page.Page_C|GetInventory (LocalVariables|GetLocal%20Attacker))))))) 2.0)) _returnvalue_2))) " damage") "Weapon/Default_Sword/Sword")
                  (Class|WorldObject|Damage(Message) (LocalVariables|GetCurrent%20Target) (Utilities|Array|MakeArray (Math|Conversions|ToFloat(Integer) (Math|Float|Ceil (* (- (+ (Variables|Default|GetDamage) (Variables|/Game/Items/WeaponObject.WeaponObject_C|GetDamage (Variables|/Game/Items/Inventory.Inventory_C|GetDominant%20Hand (Variables|/Game/Characters/Page.Page_C|GetInventory (LocalVariables|GetLocal%20Attacker)))) (LocalVariables|GetDamage%20Roll)) (/ (+ (- _total_hardness1 (Variables|/Game/Items/WeaponObject.WeaponObject_C|GetPiercing (Variables|/Game/Items/Inventory.Inventory_C|GetDominant%20Hand (Variables|/Game/Characters/Page.Page_C|GetInventory (LocalVariables|GetLocal%20Attacker))))) (Math|Float|Absolute(Float) (- _total_hardness1 (Variables|/Game/Items/WeaponObject.WeaponObject_C|GetPiercing (Variables|/Game/Items/Inventory.Inventory_C|GetDominant%20Hand (Variables|/Game/Characters/Page.Page_C|GetInventory (LocalVariables|GetLocal%20Attacker))))))) 2.0)) _returnvalue_2)))) (Utilities|Array|MakeArray (Math|Conversions|ToFloat(Integer) (Math|Float|Ceil (* (- (+ (LocalVariables|GetDamage%20Roll) (Variables|/Game/Items/WeaponObject.WeaponObject_C|GetBludgeon (Variables|/Game/Items/Inventory.Inventory_C|GetDominant%20Hand (Variables|/Game/Characters/Page.Page_C|GetInventory (LocalVariables|GetLocal%20Attacker)))) (Variables|Default|GetBludgeoning)) _total_padding1) _returnvalue_2)))) (Utilities|Array|MakeArray 0.0))
                  (Default|EventAttackTarget Attacker (LocalVariables|GetCurrent%20Target) (Variables|Default|GetHigh/Mid/Low) (Variables|Default|GetTwoH/OneHRight/OneHLeft) (Utilities|String|Append (Utilities|String|ToString(Integer) (Math|Float|Ceil (* (- (+ (Variables|Default|GetDamage) (Variables|/Game/Items/WeaponObject.WeaponObject_C|GetDamage (Variables|/Game/Items/Inventory.Inventory_C|GetDominant%20Hand (Variables|/Game/Characters/Page.Page_C|GetInventory (LocalVariables|GetLocal%20Attacker)))) (LocalVariables|GetDamage%20Roll)) (/ (+ (- _total_hardness1 (Variables|/Game/Items/WeaponObject.WeaponObject_C|GetPiercing (Variables|/Game/Items/Inventory.Inventory_C|GetDominant%20Hand (Variables|/Game/Characters/Page.Page_C|GetInventory (LocalVariables|GetLocal%20Attacker))))) (Math|Float|Absolute(Float) (- _total_hardness1 (Variables|/Game/Items/WeaponObject.WeaponObject_C|GetPiercing (Variables|/Game/Items/Inventory.Inventory_C|GetDominant%20Hand (Variables|/Game/Characters/Page.Page_C|GetInventory (LocalVariables|GetLocal%20Attacker))))))) 2.0)) _returnvalue_2))) " damage!")))))))
        (Utilities|Array|Clear (Variables|Default|GetTargetList))
        (return true)
        (else
          (Development|PrintString 0 "Not enough Targets")
          (return false))))))

(fn IsTargetValid
  (params (Target :type Object%20Object%20Reference) (Page%20attacking :type Page%20Object%20Reference))
  (bind _valid (CallFunction|IsTargetofCorrectType Target))
  (bind _witihin_range (CallFunction|IsTargetWithinRange Page%20attacking Target))
  (bind _yes_no (CallFunction|IsAttackerTarget Target Page%20attacking))
  (return (Math|Boolean|ANDBoolean _valid _witihin_range (or (not _yes_no) (Variables|Default|GetSelf%20Targettable)))))

(fn IsTargetofCorrectType
  (params (Target :type Object%20Object%20Reference))
  (for _array_element (Variables|Default|GetTargetTypes)
    (bind _type (Class|WorldObject|GetType(Message) Target))
    (if (Utilities|Enum|Equal(Enum) _array_element _type)
      (LocalVariables|SetisValid true)))
  (return (LocalVariables|GetisValid)))

(fn IsTargetWithinRange
  (params (Attacker :type Page%20Object%20Reference) (Target :type Object%20Object%20Reference))
  (bind _newparam (Class|WorldObject|GetLocation(Message) Target))
  (bind _distance (Class|WorldObject|GetDistancefromTile(Message) Attacker _newparam))
  (return (<= _distance (Variables|Default|GetRange))))

(fn Addtargets
  (params (Targets :type Array%20of%20Actor%20Object%20References))
  ;[1 1 1] Functino doesn't really make sense, should just add, logic should be elsewhere
  (for _array_element Targets
    (if (< (Utilities|Array|Length (Variables|Default|GetTargetList)) (Variables|Default|GetMax%20Targets))
      (Math|Integer|IncrementInt (LocalVariables|GetnumbTargetsAdded)
        (:%20%20
          (Utilities|Array|Add (LocalVariables|GettargetsAdded) _array_element)
          (Utilities|Array|Add (Variables|Default|GetTargetList) _array_element)
          (bind _name (Class|WorldObject|GetName(Message) _array_element))
          (Utilities|Array|Add (LocalVariables|GetLocal%20Names%20of%20Targets%20added) _name)))))
  (return (LocalVariables|GetnumbTargetsAdded) (LocalVariables|GettargetsAdded) (LocalVariables|GetLocal%20Names%20of%20Targets%20added)))

(fn IsAttackerTarget
  (params (Target :type Object%20Object%20Reference) (Attacker :type Page%20Object%20Reference))
  (return (== Target Attacker)))

(fn DoIHaveEnoughTargets
  (return (>= (Utilities|Array|Length (Variables|Default|GetTargetList)) (Variables|Default|GetMin%20Targets))))

(fn TriggerConditionMet?
  (return true))

(fn GetTargetNames
  (for _array_element (Variables|Default|GetTargetList)
    (bind _name (Class|WorldObject|GetName(Message) _array_element))
    (Utilities|Array|Add (LocalVariables|GetNames) _name))
  (return (LocalVariables|GetNames)))

(fn IsAttackBlocked?
  (params (Target :type Pawn%20Object%20Reference) (Attacker :type Pawn%20Object%20Reference) (IsDominantHand :type Boolean) (Roll :type Float%20%28single-precision%29))
  (bind _aspage (Utilities|Casting|CastToPage Attacker))
  (if IsDominantHand
    (LocalVariables|SetAccuracy%20Total (Variables|/Game/Items/WeaponObject.WeaponObject_C|GetAccuracy (Variables|/Game/Items/Inventory.Inventory_C|GetDominant%20Hand (Variables|/Game/Characters/Page.Page_C|GetInventory _aspage))))
    (else
      (LocalVariables|SetAccuracy%20Total (Variables|/Game/Items/WeaponObject.WeaponObject_C|GetAccuracy (Variables|/Game/Items/Inventory.Inventory_C|GetOffHand (Variables|/Game/Characters/Page.Page_C|GetInventory _aspage))))))
  (bind _aspage_2 (Utilities|Casting|CastToPage Target))
  (Utilities|IsValid (Variables|/Game/Characters/Page.Page_C|GetcurrentStance _aspage_2)
    (:Is%20Valid
      (LocalVariables|SetGuard%20Total (Variables|/Game/BluePrints/Stances/Stance.Stance_C|GetHigh%20Guard (Variables|/Game/Characters/Page.Page_C|GetcurrentStance _aspage_2))))
    (:Is%20Not%20Valid
      _))
  (bind _output_get (LocalVariables|SetGuard%20Total (+ (LocalVariables|GetGuard%20Total) (Variables|/Game/Items/WeaponObject.WeaponObject_C|GetGuard (Variables|/Game/Items/Inventory.Inventory_C|GetDominant%20Hand (Variables|/Game/Characters/Page.Page_C|GetInventory _aspage_2))) (Variables|/Game/Items/WeaponObject.WeaponObject_C|GetGuard (Variables|/Game/Items/Inventory.Inventory_C|GetOffHand (Variables|/Game/Characters/Page.Page_C|GetInventory _aspage_2))) 1e+01)))
  (Development|PrintString 0 (Utilities|String|Append "Guard Total is: " (Utilities|String|ToString(Float) _output_get) " Accuracy Total: " (Utilities|String|ToString(Float) (+ Roll (LocalVariables|GetAccuracy%20Total) (Variables|Default|GetAccuracy)))))
  (if (< _output_get (+ Roll (LocalVariables|GetAccuracy%20Total) (Variables|Default|GetAccuracy)))
    (Development|PrintString 0 "Attack/Is Attack Blocked/ Attack was not blocked")
    (return false (Utilities|String|Append "Guard Total is: " (Utilities|String|ToString(Float) _output_get) " Accuracy Total: " (Utilities|String|ToString(Float) (+ Roll (LocalVariables|GetAccuracy%20Total) (Variables|Default|GetAccuracy)))))
    (else
      (Development|PrintString 0 "Attack/Is Attack Blocked/ Attack was blocked")
      (return true (Utilities|String|Append "Guard Total is: " (Utilities|String|ToString(Float) _output_get) " Accuracy Total: " (Utilities|String|ToString(Float) (+ Roll (LocalVariables|GetAccuracy%20Total) (Variables|Default|GetAccuracy))))))))

(fn IsAttackDodged?
  (params (Attacker :type Page%20Object%20Reference) (Target :type Page%20Object%20Reference) (UseDominant :type Boolean) (Roll :type Float%20%28single-precision%29))
  (bind _returnvalue (Utilities|String|ToString(Float) Roll))
  (bind _accuracy (Variables|Default|GetAccuracy))
  (bind _inventory (Variables|/Game/Characters/Page.Page_C|GetInventory Attacker))
  (bind _stats (Variables|/Game/Characters/Page.Page_C|GetStats Target))
  (bind _dexterity (Utilities|Struct|BreakOStatBlockStruct _stats))
  (bind _returnvalue_2 (Utilities|String|ToString(Float) _accuracy))
  (bind _returnvalue_3 (Utilities|String|ToString(Float) _dexterity))
  (bind _returnvalue_4 (Utilities|String|Append " Die Roll: " _returnvalue "Accuracy from attack" _returnvalue_2 " Accuracy From weapon" "Enemies Dexterity" _returnvalue_3))
  (if UseDominant
    (LocalVariables|SetLocal%20Accuracy (Variables|/Game/Items/WeaponObject.WeaponObject_C|GetAccuracy (Variables|/Game/Items/Inventory.Inventory_C|GetDominant%20Hand _inventory)))
    (else
      (LocalVariables|SetLocal%20Accuracy (Variables|/Game/Items/WeaponObject.WeaponObject_C|GetAccuracy (Variables|/Game/Items/Inventory.Inventory_C|GetOffHand _inventory)))))
  (Development|PrintString 0 _returnvalue_4)
  (if (> (+ Roll (+ (LocalVariables|GetLocal%20Accuracy) (Variables|Default|GetAccuracy))) _dexterity)
    (return false _returnvalue_4)
    (else
      (Development|PrintString 0 "Attack/Does Attack Hit/Attack misses the target completely")
      (return true _returnvalue_4))))

(fn IsHitCritical?
  (params (Attacker :type Page%20Object%20Reference) (Target :type Page%20Object%20Reference) (IsDominant :type Boolean) (Roll :type Float%20%28single-precision%29))
  (bind _inventory (Variables|/Game/Characters/Page.Page_C|GetInventory Attacker))
  (bind _total_coverage1 (Default|GetDefensiveStats (Variables|/Game/Characters/Page.Page_C|GetInventory Target)))
  (if IsDominant
    (LocalVariables|SetLocal%20Accuracy (Variables|/Game/Items/WeaponObject.WeaponObject_C|GetAccuracy (Variables|/Game/Items/Inventory.Inventory_C|GetDominant%20Hand _inventory)))
    (else
      (LocalVariables|SetLocal%20Accuracy (Variables|/Game/Items/WeaponObject.WeaponObject_C|GetAccuracy (Variables|/Game/Items/Inventory.Inventory_C|GetOffHand _inventory)))))
  (if (< _total_coverage1 (+ Roll (+ (LocalVariables|GetLocal%20Accuracy) (Variables|Default|GetAccuracy))))
    (Development|PrintString 0 "Attack/IsHitCiritcal/Attack is an excellent hit!")
    (return true)
    (else
      (Development|PrintString 0 "Attack/IsHitCiritcal/Attack is just a regular hit")
      (return false))))

(fn GetDeflectionModifier
  (params (Attacker :type Page%20Object%20Reference) (Target :type Page%20Object%20Reference) (IsDominant :type Boolean) (Roll :type Float%20%28single-precision%29))
  (bind _inventory (Variables|/Game/Characters/Page.Page_C|GetInventory Attacker))
  (bind _dominant_hand (Variables|/Game/Items/Inventory.Inventory_C|GetDominant%20Hand _inventory))
  (bind _offhand (Variables|/Game/Items/Inventory.Inventory_C|GetOffHand _inventory))
  (bind _total_deflection1 (Default|GetDefensiveStats (Variables|/Game/Characters/Page.Page_C|GetInventory Target)))
  (LocalVariables|SetLocal%20Deflection _total_deflection1)
  (if IsDominant
    (LocalVariables|SetLocal%20Accuracy (+ (Variables|/Game/Items/WeaponObject.WeaponObject_C|GetAccuracy _dominant_hand) (Variables|/Game/Items/WeaponObject.WeaponObject_C|GetContact _dominant_hand)))
    (else
      (LocalVariables|SetLocal%20Accuracy (+ (Variables|/Game/Items/WeaponObject.WeaponObject_C|GetAccuracy _offhand) (Variables|/Game/Items/WeaponObject.WeaponObject_C|GetContact _offhand)))))
  (return (/ (- (+ Roll (+ (LocalVariables|GetLocal%20Accuracy) (Variables|Default|GetAccuracy))) (LocalVariables|GetLocal%20Deflection)) (+ Roll (+ (LocalVariables|GetLocal%20Accuracy) (Variables|Default|GetAccuracy))))))

(fn BuildAttackfromStruct
  (params (Struct%20in :type O%20Attack%20Struct%20Structure))
  (bind (_key _classkey _mintargets _maxtargets _range _initiativecost _staminacost _vitalitycost _manacost _selftargettable _accuracy _piercing _damage _contact _bludgeon _mainhandrequirements _offhandrequirements _targettypes _widgetkey _attackheight _wieldtype) (Utilities|Struct|BreakOAttackStruct Struct%20in))
  (Variables|Default|SetSerialized%20Data Struct%20in)
  (Variables|Default|SetAttack%20Name _key)
  (Variables|Default|SetMin%20Targets _mintargets)
  (Variables|Default|SetMax%20Targets _maxtargets)
  (Variables|Default|SetRange _range)
  (Variables|Default|SetStamina%20Cost (Math|Float|Truncate _staminacost))
  (Variables|Default|SetSelf%20Targettable _selftargettable)
  (Variables|Default|SetAccuracy _accuracy)
  (Variables|Default|SetContact _contact)
  (Variables|Default|SetPiercing _piercing)
  (Variables|Default|SetDamage _damage)
  (Variables|Default|SetWidget%20Key _widgetkey)
  (Variables|Default|SetBludgeoning _bludgeon)
  (for _array_element _mainhandrequirements
    (Utilities|Array|Add (Variables|Default|GetMainHandRequirements) (Utilities|Enum|ByteToEnumWeaponTypes (Math|Conversions|ToByte(Integer) _array_element))))
  (for _array_element_2 _offhandrequirements
    (Utilities|Array|Add (Variables|Default|GetOffHandRequirements) (Utilities|Enum|ByteToEnumWeaponTypes (Math|Conversions|ToByte(Integer) _array_element_2))))
  (for _array_element_3 _targettypes
    (Utilities|Array|Add (Variables|Default|GetTargetTypes) (Utilities|Enum|ByteToEnumWorldObjectTypes (Math|Conversions|ToByte(Integer) _array_element_3))))
  (Variables|Default|SetInitiative%20Cost _initiativecost)
  (Variables|Default|SetHigh/Mid/Low (Utilities|Enum|ByteToEnumAttackHeight (Math|Conversions|ToByte(Integer) _attackheight)))
  (Variables|Default|SetTwoH/OneHRight/OneHLeft (Utilities|Enum|ByteToEnumAttackWieldType (Math|Conversions|ToByte(Integer) _wieldtype))))