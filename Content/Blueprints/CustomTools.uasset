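; CustomTools is a helper function collection for a tile-grid game with initiative-based movement.
; FindPathCaller wraps FindPath, a recursive depth-first search for the cheapest route around occupied tiles, using a hardcoded cost cutoff that ignores CostLimit.
; GetSubsectionOfPath trims paths to available initiative, and other helpers map world positions to tiles through PNPGameState.
; Utilities cover neighbor checks, facing and angle math, mouse-anchored widget placement and unique array merging; two functions are empty stubs.
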(fn AreTilesNeighbors
  (params (Potential%20Neighbor :type BP%20Tile%20Object%20Reference) (Tile :type BP%20Tile%20Object%20Reference))
  (bind _x_coordinate (Variables|/Game/Tiles/BPTile.BPTile_C|GetX%20Coordinate Tile))
  (bind _y_coordinate (Variables|/Game/Tiles/BPTile.BPTile_C|GetY%20Coordinate Tile))
  (bind _x_coordinate_2 (Variables|/Game/Tiles/BPTile.BPTile_C|GetX%20Coordinate Potential%20Neighbor))
  (bind _y_coordinate_2 (Variables|/Game/Tiles/BPTile.BPTile_C|GetY%20Coordinate Potential%20Neighbor))
  (bind _returnvalue (== _x_coordinate_2 _x_coordinate))
  (bind _returnvalue_2 (== _y_coordinate_2 _y_coordinate))
  (return (and _returnvalue (== (+ _y_coordinate_2 1) _y_coordinate)) (and _returnvalue (== (- _y_coordinate_2 1) _y_coordinate)) (and _returnvalue_2 (== (- _x_coordinate_2 1) _x_coordinate)) (and _returnvalue_2 (== (+ _x_coordinate_2 1) _x_coordinate))))

(fn GetPage
  (bind _aspage (Utilities|Casting|CastToPage (Pawn|GetControlledPawn (Game|GetPlayerController 0))))
  (return _aspage))

(fn CallClickHandler
  (params (Object%20Reference :type Object%20Object%20Reference))
  (bind _ascharacter (Utilities|Casting|CastToCharacter (Game|GetPlayerController 0)))
  (Default|ClickHandler _ascharacter Object%20Reference))

(fn FindPlaceforWidget
  (params (Widget%20 :type Float%20%28single-precision%29))
  (bind _returnvalue (Class|WidgetLayoutLibrary|GetMousePositiononViewport))
  (bind _returnvalue_2 (Class|WidgetLayoutLibrary|GetViewportWidgetGeometry))
  (if (< (- (.Y (Math|Vector2D|BreakVector2D (Class|SlateBlueprintLibrary|GetLocalSize _returnvalue_2))) (+ (.Y (Math|Vector2D|BreakVector2D _returnvalue)) Widget%20)) 0.0)
    (return (+ _returnvalue (Math|Vector2D|MakeVector2D 0.0 (- (.Y (Math|Vector2D|BreakVector2D (Class|SlateBlueprintLibrary|GetLocalSize _returnvalue_2))) (+ (.Y (Math|Vector2D|BreakVector2D _returnvalue)) Widget%20)))))
    (else
      (return _returnvalue))))

(fn FindPath
  (params (Destination :type BP%20Tile%20Object%20Reference) (PathSoFar :type Array%20of%20BP%20Tile%20Object%20References) (MovementSpentSoFar :type Float%20%28single-precision%29) (Tile%20Being%20Checked :type BP%20Tile%20Object%20Reference) (Cost%20Limit :type Float%20%28single-precision%29))
  (LocalVariables|SetCost%20to%20Return 1e+02)
  (LocalVariables|SetDirection (Utilities|Array|MakeArray "NewEnumerator0" "NewEnumerator1" "NewEnumerator2" "NewEnumerator3"))
  (if (== Destination Tile%20Being%20Checked)
    (Development|PrintString 0 "CustomTools/FindPath/You have found your path!" false false)
    (return PathSoFar MovementSpentSoFar)
    (else
      (if (and (Variables|/Game/Tiles/BPTile.BPTile_C|GetOccupied Tile%20Being%20Checked) (not (== Tile%20Being%20Checked (Utilities|Array|Get(acopy) PathSoFar))))
        _
        (elif (> MovementSpentSoFar 1e+01)
          _
          (else
            (for _array_element (LocalVariables|GetDirection)
              (bind _output (Default|GetNeighbor Tile%20Being%20Checked _array_element))
              (Utilities|IsValid _output
                (:Is%20Valid
                  (if (not (Utilities|Array|ContainsItem PathSoFar _output))
                    (bind _output_get (LocalVariables|SetNew%20Path PathSoFar))
                    (Utilities|Array|Add _output_get _output)
                    (bind (_pathout _costout) (CallFunction|FindPath Destination (LocalVariables|GetNew%20Path) (+ MovementSpentSoFar (Variables|/Game/Tiles/BPTile.BPTile_C|GetmovementCost Tile%20Being%20Checked)) _output Cost%20Limit))
                    (if (< _costout (LocalVariables|GetCost%20to%20Return))
                      (LocalVariables|SetCost%20to%20Return _costout)
                      (LocalVariables|SetPath%20to%20Return _pathout))
                    (else
                      (Development|PrintString 0 "CustomTools/FindPath/Path already contains this tile" false false))))
                (:Is%20Not%20Valid
                  (Development|PrintString 0 "CustomTools/FIndPath/Your Neighbot is not valid" false false))))
            (return (LocalVariables|GetPath%20to%20Return) (LocalVariables|GetCost%20to%20Return)))))
      (return 0 15.0))))

(fn GetDistanceBetweenTiles
  (params (Tile%201 :type BP%20Tile%20Object%20Reference) (Tile%202 :type BP%20Tile%20Object%20Reference))
  (bind (_pathout _costout) (CallFunction|FindPath Tile%202 (Utilities|Array|MakeArray Tile%201) 0.0 Tile%201 15.0))
  (Development|PrintString 0 (Utilities|String|Append "Cost out is: " (Utilities|String|ToString(Float) _costout)))
  (return (- (Utilities|Array|Length _pathout) 1)))

(fn GetPositionforWidget
  (params (Size :type Float%20%28single-precision%29))
  (bind _returnvalue (Class|WidgetLayoutLibrary|GetMousePositiononViewport))
  (bind _returnvalue_2 (Class|WidgetLayoutLibrary|GetViewportWidgetGeometry))
  (if (< (- (.Y (Math|Vector2D|BreakVector2D (Class|SlateBlueprintLibrary|GetLocalSize _returnvalue_2))) (+ (.Y (Math|Vector2D|BreakVector2D _returnvalue)) Size)) 0.0)
    (return (+ _returnvalue (Math|Vector2D|MakeVector2D 0.0 (- (.Y (Math|Vector2D|BreakVector2D (Class|SlateBlueprintLibrary|GetLocalSize _returnvalue_2))) (+ (.Y (Math|Vector2D|BreakVector2D _returnvalue)) Size)))))
    (else
      (return _returnvalue))))

(fn AppendUniqueObjects
  (params (Array%201 :type Array%20of%20Object%20Object%20References) (Array%202 :type Array%20of%20Object%20Object%20References))
  (LocalVariables|SetArray%20out Array%201)
  (for _array_element Array%202
    (Utilities|Array|AddUnique (LocalVariables|GetArray%20out) _array_element))
  (return (LocalVariables|GetArray%20out)))

(fn GetLabelfromClass
  (params (Object :type Navigation%20Object%20Base%20Class%20Reference)))

(fn AppendUniqeStanceClasses
  (params (Array%201 :type Array%20of%20Stance%20Class%20References) (Array%202 :type Array%20of%20Stance%20Class%20References))
  (LocalVariables|SetClasses%20out Array%201)
  (for _array_element Array%202
    (Utilities|Array|AddUnique (LocalVariables|GetClasses%20out) _array_element))
  (return (LocalVariables|GetClasses%20out)))

(fn FindActorsLocation
  (params (Target :type Actor%20Object%20Reference))
  (bind _returnvalue (Transformation|GetActorTransform Target))
  (bind _location (Math|Transform|BreakTransform _returnvalue))
  (bind (_x _y) (Math|Vector|BreakVector _location))
  (bind _aspnpgame_state (Utilities|Casting|CastToPNPGameState (Game|GetGameState)))
  (bind _output (Default|GetTile _aspnpgame_state (Math|Float|Truncate (/ _x (Variables|/Game/States/PNPGameState.PNPGameState_C|GetTile%20width _aspnpgame_state))) (Math|Float|Truncate (/ _y (Variables|/Game/States/PNPGameState.PNPGameState_C|GetTile%20length _aspnpgame_state)))))
  (return _output))

(fn SortbyInitiative
  (params (NewParam :type Object%20Object%20Reference)))

(fn GetSubsectionOfPath
  (params (Path%20in :type Array%20of%20BP%20Tile%20Object%20References) (Available%20Initiative :type Float%20%28single-precision%29))
  (bind _array_element (Utilities|Array|ForEachLoopwithBreak Path%20in :!label _label)
    (:LoopBody
      (if (<= (+ (Variables|/Game/Tiles/BPTile.BPTile_C|GetmovementCost _array_element) (LocalVariables|GetInitiative%20Sum)) Available%20Initiative)
        (LocalVariables|SetInitiative%20Sum (+ (Variables|/Game/Tiles/BPTile.BPTile_C|GetmovementCost _array_element) (LocalVariables|GetInitiative%20Sum)))
        (Utilities|Array|Add (LocalVariables|GetPath%20Out) _array_element)
        (else
          (goto _label Break))))
    (:Completed
      (return (LocalVariables|GetPath%20Out)))))

(fn FindPathCaller
  (params (Destination :type BP%20Tile%20Object%20Reference) (Where%20you%20are :type BP%20Tile%20Object%20Reference) (Max%20path%20cost :type Float%20%28single-precision%29))
  (Utilities|IsValid Destination
    (:Is%20Valid
      (bind (_pathout _costout) (CallFunction|FindPath Destination (Utilities|Array|MakeArray Where%20you%20are) 0.0 Where%20you%20are Max%20path%20cost))
      (bind _output_get (LocalVariables|SetPath _pathout))
      (Utilities|Array|RemoveIndex _output_get)
      (return (LocalVariables|GetPath) _costout))
    (:Is%20Not%20Valid
      (return 0 0.0))))

(fn GetAngleBetweenVectors
  (params (Vector1 :type Vector%202D%20Structure) (Vector2 :type Vector%202D%20Structure))
  (return (Class|KismetMathLibrary|DegAcos (/ (Math|Vector2D|DotProduct(2D) Vector1 Vector2) (* (Math|Float|Absolute(Float) (Math|Vector2D|Vector2DLength Vector1)) (Math|Float|Absolute(Float) (Math|Vector2D|Vector2DLength Vector2)))))))

(fn FacingtoVector
  (params (Facing :type Directions%20Enum :default "NewEnumerator0"))
  (switch Utilities|FlowControl|Switch|SwitchonDirections Facing
    (:NewEnumerator0
      (return "(X=0.000000,Y=-1.000000)"))
    (:NewEnumerator1
      (return "(X=1.000000,Y=0.000000)"))
    (:NewEnumerator2
      (return "(X=0.000000,Y=1.000000)"))
    (:NewEnumerator3
      (return "(X=-1.000000,Y=0.000000)"))))

(fn GetTileWidthtoIncrementby
  (params (Angle :type Float%20%28single-precision%29) (Tile%20Width :type Float%20%28single-precision%29))
  (return (+ (Math|Float|Absolute(Float) (* 0.41 (Math|Trig|Sin(Degrees) (* Angle 2.0)) Tile%20Width)) Tile%20Width)))

(fn GetTilefromLocation
  (params (X :type Float%20%28single-precision%29) (Y :type Float%20%28single-precision%29))
  (bind _aspnpgame_state (Utilities|Casting|CastToPNPGameState (Game|GetGameState)))
  (bind _output (Default|GetTile _aspnpgame_state (Math|Float|Truncate (/ X (Variables|/Game/States/PNPGameState.PNPGameState_C|GetTile%20width _aspnpgame_state))) (Math|Float|Truncate (/ Y (Variables|/Game/States/PNPGameState.PNPGameState_C|GetTile%20length _aspnpgame_state)))))
  (return _output))