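; Stance Blueprint that holds the data for one combat stance: attacks, allowed main-hand and off-hand weapon types, high, middle and low guards, and combat modifiers.
; Its single function, BuildStanceFromStruct, initializes the stance by copying each field of a passed-in struct into the matching variable.
; The modifiers cover accuracy, damage, piercing, bludgeon and contact, with no further logic in the graph.
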(fn BuildStancefromStruct
  (params (Struct :type O%20Stance%20Struct%20Structure))
  (bind (_key _classkey _attacks _mainhandweapontypes _offhandweapontypes _highguard _midguard _lowguard _accuracymodifier _damagemodifier _piercingmodifier _bludgeonmodifier _contactmodifier) (Utilities|Struct|BreakOStanceStruct Struct))
  (Variables|Default|SetAttacks _attacks)
  (Variables|Default|SetMainhandTypes _mainhandweapontypes)
  (Variables|Default|SetOffHandTypes _offhandweapontypes)
  (Variables|Default|SetHigh%20Guard _highguard)
  (Variables|Default|SetMiddle%20Guard _midguard)
  (Variables|Default|SetLow%20Guard _lowguard)
  (Variables|Default|SetAccuracy%20Modifier _accuracymodifier)
  (Variables|Default|SetDamage%20Modifier _damagemodifier)
  (Variables|Default|SetPiercing%20Modifier _piercingmodifier)
  (Variables|Default|SetBludgeon%20modifier _bludgeonmodifier)
  (Variables|Default|SetContact%20Modifier _contactmodifier)
  (return))