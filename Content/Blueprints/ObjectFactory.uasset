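; ObjectFactory creates game data objects by key: weapons, items, armor, stances, stat blocks, attacks and enchantments.
; Most functions look up a struct, construct an object with the factory as Outer, then initialize it through a build call.
; Items switch on the struct key to pick a Key subclass or generic ItemObject.
; Attacks and enchantments ignore their key and return uninitialized objects.
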(fn ConstructWeapon
  (params (Key :type String))
  (bind _returnvalue (Class|DataLoader|GetWeaponStruct Key))
  (bind _returnvalue_2 (Game|ConstructObjectfromClass "/Game/Items/WeaponObject.WeaponObject_C" self))
  (bind _output_get (LocalVariables|SetLocal%20Weapon _returnvalue_2))
  (Default|BuildWeaponfromStruct _output_get _returnvalue)
  (return (LocalVariables|GetLocal%20Weapon)))

(fn ConstructItem
  (params (Key :type String))
  (bind _returnvalue (Class|DataLoader|GetItemStruct Key))
  (switch string (.key (Utilities|Struct|BreakOItemStruct _returnvalue))
    (:Default
      (bind _returnvalue_2 (Game|ConstructObjectfromClass "/Game/Items/ItemObject.ItemObject_C" self))
      (LocalVariables|SetItem%20Being%20constructed _returnvalue_2))
    (:Key
      (bind _returnvalue_3 (Game|ConstructObjectfromClass "/Game/Items/Key.Key_C" self))
      (LocalVariables|SetItem%20Being%20constructed _returnvalue_3)))
  (Default|BuildfromStruct (LocalVariables|GetItem%20Being%20constructed) _returnvalue)
  (return (LocalVariables|GetItem%20Being%20constructed)))

(fn ConstructAttack
  (params (Key :type String))
  (bind _returnvalue (Game|ConstructObjectfromClass "/Game/BluePrints/Attacks/Attack.Attack_C" self))
  (return _returnvalue))

(fn ConstructStance
  (params (Key :type String))
  (bind _returnvalue (Class|DataLoader|GetStanceStruct Key))
  (switch string (.classKey (Utilities|Struct|BreakOStanceStruct _returnvalue))
    (:Default
      (bind _returnvalue_2 (Game|ConstructObjectfromClass "/Game/BluePrints/Stances/Stance.Stance_C" self))
      (bind _output_get (LocalVariables|SetStance _returnvalue_2))
      (Default|BuildStancefromStruct _output_get _returnvalue)
      (return (LocalVariables|GetStance)))))

(fn ConstructArmor
  (params (Key :type String))
  (bind _returnvalue (Class|DataLoader|GetArmorStruct Key))
  (bind _returnvalue_2 (Game|ConstructObjectfromClass "/Game/Items/ArmorObject.ArmorObject_C" self))
  (bind _armor_out (Default|BuildArmorfromStruct _returnvalue_2 _returnvalue))
  (return _armor_out))

(fn ConstructEnchantment
  (params (Key :type String))
  (bind _returnvalue (Game|ConstructObjectfromClass "/Game/BluePrints/Enchantments/Enchantment.Enchantment_C" self))
  (return _returnvalue))

(fn ConstructStatBlock
  (params (Key :type String))
  (bind _returnvalue (Class|DataLoader|GetStatBlock Key))
  (bind _returnvalue_2 (Game|ConstructObjectfromClass "/Game/CharacterStats.CharacterStats_C" self))
  (bind _output_get (LocalVariables|SetLocal%20Stat%20Block _returnvalue_2))
  (Default|BuildStatsfromStatBlock _output_get _returnvalue)
  (return (LocalVariables|GetLocal%20Stat%20Block)))