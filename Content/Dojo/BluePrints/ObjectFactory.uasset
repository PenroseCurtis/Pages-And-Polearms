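; ObjectFactory is a Blueprint that creates item and weapon objects from struct data looked up by key.
; ConstructItem picks a class from the struct's ClassKey, either Key or a default ItemObject, then fills the new object through BuildFromStruct and returns it.
; ConstructWeapon is unfinished: it creates a WeaponObject and fetches its struct, but neither applies the data nor returns the object.
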(fn ConstructWeapon
  (params (Key :type String))
  (Game|ConstructObjectfromClass "/Game/Dojo/Items/WeaponObject.WeaponObject_C" self)
  (bind _returnvalue (Class|DataLoader|GetWeaponStruct Key)))

(fn ConstructItem
  (params (Key :type String))
  (bind _returnvalue (Class|DataLoader|GetItemStruct Key))
  (switch string (.classKey (Utilities|Struct|BreakOItemStruct _returnvalue))
    (:Default
      (bind _returnvalue_2 (Game|ConstructObjectfromClass "/Game/Dojo/Items/ItemObject.ItemObject_C" self))
      (LocalVariables|SetItem%20Being%20constructed _returnvalue_2))
    (:Key
      (bind _returnvalue_3 (Game|ConstructObjectfromClass "/Game/Dojo/Items/Key.Key_C" self))
      (LocalVariables|SetItem%20Being%20constructed _returnvalue_3)))
  (Default|BuildfromStruct (LocalVariables|GetItem%20Being%20constructed) _returnvalue)
  (return (LocalVariables|GetItem%20Being%20constructed)))