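; Scratch is an attack Blueprint in the Dojo game that damages the vitality, stamina and mana of its targets.
; It overrides Attack, runs the parent implementation first and returns that result.
; When the parent succeeds, it sends a DamageMessage with fixed amounts to every entry in TargetList.
; Debug prints report the target count and each hit.
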(fn Attack
  (params (Attacker :type Page%20Object%20Reference))
  (bind _array (Utilities|Array|MakeArray 1e+02))
  (Development|PrintString 0 (Utilities|String|Append "Scratch/Attack/Starting scratch. The length of my target list is: " (Utilities|String|ToString(Integer) (Utilities|Array|Length (Variables|Default|GetTargetList)))))
  (bind _attack_completed (|CallParentFunction Attacker))
  (if _attack_completed
    (for _array_element (Variables|Default|GetTargetList)
      (Class|WorldObject|Damage(Message) _array_element _array _array _array)
      (Development|PrintString 0 "Scratch/Attack/Damaging target!")))
  (return _attack_completed))