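; Punch attack that overrides a parent Attack and, if the parent succeeds, resolves a dominant-hand strike on each Page in the target list.
; A millisecond-seeded hit roll feeds dodge, block and deflection checks.
; Damage roll plus Piercing or Bludgeon is scaled by deflection, reduced by hardness or padding, then sent as Vitality and Stamina damage.
; Afterwards it clears the targets and the attacker's pending attack.
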(fn Attack
  (params (Attacker :type Page%20Object%20Reference))
  (bind _returnvalue (Math|DateTime|Now))
  (bind _inventory (Variables|/Game/Dojo/Page.Page_C|GetInventory Attacker))
  (bind _returnvalue_2 (Math|DateTime|GetMillisecond _returnvalue))
  (bind _dominant_hand (Variables|/Game/Dojo/Items/Inventory.Inventory_C|GetDominant%20Hand _inventory))
  (bind _returnvalue_3 (Math|Random|MakeRandomStream _returnvalue_2))
  (bind _attack_completed (|CallParentFunction Attacker))
  (LocalVariables|SetHit%20Roll (Math|Random|RandomFloatinRangefromStream 1.0 2e+01 _returnvalue_3))
  (LocalVariables|SetDamage%20Roll (Math|Random|RandomFloatinRangefromStream 1.0 (Variables|Default|GetDamage) _returnvalue_3))
  (if _attack_completed
    (for _array_element (Variables|Default|GetTargetList)
      (bind _aspage (Utilities|Casting|CastToPage _array_element))
      (bind _isdodged (CallFunction|IsAttackDodged? Attacker _aspage true (LocalVariables|GetHit%20Roll)))
      (if (not _isdodged)
        (bind _newparam (CallFunction|IsAttackBlocked? _aspage Attacker true (LocalVariables|GetHit%20Roll)))
        (if (not _newparam)
          (bind _returnvalue_4 (CallFunction|GetDeflectionModifier Attacker _aspage true (LocalVariables|GetHit%20Roll)))
          (bind (_total_coverage1 _total_padding1 _total_hardness1) (Default|GetDefensiveStats (Variables|/Game/Dojo/Page.Page_C|GetInventory _aspage)))
          (Development|PrintString 0 (Utilities|String|Append "Deflection Modifier: " (Utilities|String|ToString(Float) _returnvalue_4) "Damage out" (Utilities|String|ToString(Float) (- (* (+ (LocalVariables|GetDamage%20Roll) (Variables|/Game/Dojo/Items/WeaponObject.WeaponObject_C|GetPiercing _dominant_hand)) _returnvalue_4) _total_hardness1)) " Bludgeon out" (Utilities|String|ToString(Float) (- (* (+ (LocalVariables|GetDamage%20Roll) (Variables|/Game/Dojo/Items/WeaponObject.WeaponObject_C|GetBludgeon _dominant_hand)) _returnvalue_4) _total_padding1))))
          (Class|WorldObject|Damage(Message) _aspage (Utilities|Array|MakeArray (- (* (+ (LocalVariables|GetDamage%20Roll) (Variables|/Game/Dojo/Items/WeaponObject.WeaponObject_C|GetPiercing _dominant_hand)) _returnvalue_4) _total_hardness1)) (Utilities|Array|MakeArray (- (* (+ (LocalVariables|GetDamage%20Roll) (Variables|/Game/Dojo/Items/WeaponObject.WeaponObject_C|GetBludgeon _dominant_hand)) _returnvalue_4) _total_padding1)) (Utilities|Array|MakeArray 0.0)))))
    (Utilities|Array|Clear (Variables|Default|GetTargetList))
    (Variables|/Game/Dojo/Page.Page_C|SetpendingAttack Attacker 0)
    (return true)
    (else
      (return _attack_completed))))