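; Attack for Page characters in a tile-based, dice-roll combat system, handling targeting and hit-resolution math.
; Targets are added up to a cap, then filtered by class, range and self-targeting; Attack only checks the minimum count and prints.
; Separate checks compare roll plus weapon and attack accuracy against guard, Dexterity or armor coverage for block, dodge and critical.
; A deflection modifier also factors in weapon contact; TriggerConditionMet always returns true.
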(fn GetValidTargets
  (params (Targets :type Array%20of%20Object%20Object%20References) (Attacker :type Page%20Object%20Reference))
  (Utilities|Array|Clear (LocalVariables|GetLocal%20targets))
  (for _array_element Targets
    (bind _valid (CallFunction|IsTargetValid _array_element Attacker))
    (if _valid
      (Utilities|Array|Add (LocalVariables|GetLocal%20targets) _array_element)))
  (return (LocalVariables|GetLocal%20targets)))

(fn Attack
  (params (Attacker :type Page%20Object%20Reference))
  (bind _local_targets1 (CallFunction|GetValidTargets (Variables|Default|GetTargetList) Attacker))
  (Variables|Default|SetTargetList _local_targets1)
  (bind _returnvalue (CallFunction|DoIHaveEnoughTargets))
  (if _returnvalue
    (Development|PrintString 0 "Attack!")
    (return true)
    (else
      (Development|PrintString 0 "Not enough Targets")
      (return false))))

(fn IsTargetValid
  (params (Target :type Object%20Object%20Reference) (Page%20attacking :type Page%20Object%20Reference))
  (bind _valid (CallFunction|IsTargetofCorrectType Target))
  (bind _witihin_range (CallFunction|IsTargetWithinRange Page%20attacking Target))
  (bind _yes_no (CallFunction|IsAttackerTarget Target Page%20attacking))
  (return (Math|Boolean|ANDBoolean _valid _witihin_range (or (not _yes_no) (Variables|Default|GetSelf%20Targettable)))))

(fn IsTargetofCorrectType
  (params (Target :type Object%20Object%20Reference))
  (for _array_element (Variables|Default|GetTargetTypes)
    (if (Utilities|ClassIsChildOf (Utilities|GetClass Target) _array_element)
      (LocalVariables|SetisValid true)))
  (return (LocalVariables|GetisValid)))

(fn IsTargetWithinRange
  (params (Attacker :type Page%20Object%20Reference) (Target :type Object%20Object%20Reference))
  (bind _newparam (Class|WorldObject|GetLocation(Message) Target))
  (bind _distance (Class|WorldObject|GetDistancefromTile(Message) Attacker _newparam))
  (return (<= _distance (Variables|Default|GetRange))))

(fn Addtargets
  (params (Targets :type Array%20of%20Object%20Object%20References))
  (for _array_element Targets
    (if (< (Utilities|Array|Length (Variables|Default|GetTargetList)) (Variables|Default|GetMax%20Targets))
      (Math|Integer|IncrementInt (LocalVariables|GetnumbTargetsAdded)
        (:%20%20
          (Utilities|Array|Add (LocalVariables|GettargetsAdded) _array_element)
          (Utilities|Array|Add (Variables|Default|GetTargetList) _array_element)))))
  (return (LocalVariables|GetnumbTargetsAdded) (LocalVariables|GettargetsAdded)))

(fn IsAttackerTarget
  (params (Target :type Object%20Object%20Reference) (Attacker :type Page%20Object%20Reference))
  (return (== Target Attacker)))

(fn DoIHaveEnoughTargets
  (return (>= (Utilities|Array|Length (Variables|Default|GetTargetList)) (Variables|Default|GetMin%20Targets))))

(fn TriggerConditionMet?
  (return true))

(fn GetTargetNames
  (for _array_element (Variables|Default|GetTargetList)
    (bind _name (Class|WorldObject|GetName(Message) _array_element))
    (Utilities|Array|Add (LocalVariables|GetNames) _name))
  (return (LocalVariables|GetNames)))

(fn IsAttackBlocked?
  (params (Target :type Pawn%20Object%20Reference) (Attacker :type Pawn%20Object%20Reference) (IsDominantHand :type Boolean) (Roll :type Float%20%28single-precision%29))
  (bind _aspage (Utilities|Casting|CastToPage Attacker))
  (if IsDominantHand
    (LocalVariables|SetAccuracy%20Total (Variables|/Game/Dojo/Items/WeaponObject.WeaponObject_C|GetAccuracy (Variables|/Game/Dojo/Items/Inventory.Inventory_C|GetDominant%20Hand (Variables|/Game/Dojo/Page.Page_C|GetInventory _aspage))))
    (else
      (LocalVariables|SetAccuracy%20Total (Variables|/Game/Dojo/Items/WeaponObject.WeaponObject_C|GetAccuracy (Variables|/Game/Dojo/Items/Inventory.Inventory_C|GetOffHand (Variables|/Game/Dojo/Page.Page_C|GetInventory _aspage))))))
  (bind _aspage_2 (Utilities|Casting|CastToPage Target))
  (Utilities|IsValid (Variables|/Game/Dojo/Page.Page_C|GetcurrentStance _aspage_2)
    (:Is%20Valid
      (LocalVariables|SetGuard%20Total (Variables|/Game/Dojo/BluePrints/Stances/Stance.Stance_C|GetHigh%20Guard (Variables|/Game/Dojo/Page.Page_C|GetcurrentStance _aspage_2))))
    (:Is%20Not%20Valid
      _))
  (bind _output_get (LocalVariables|SetGuard%20Total (+ (LocalVariables|GetGuard%20Total) (Variables|/Game/Dojo/Items/WeaponObject.WeaponObject_C|GetGuard (Variables|/Game/Dojo/Items/Inventory.Inventory_C|GetDominant%20Hand (Variables|/Game/Dojo/Page.Page_C|GetInventory _aspage_2))) (Variables|/Game/Dojo/Items/WeaponObject.WeaponObject_C|GetGuard (Variables|/Game/Dojo/Items/Inventory.Inventory_C|GetOffHand (Variables|/Game/Dojo/Page.Page_C|GetInventory _aspage_2))) 1e+01)))
  (Development|PrintString 0 (Utilities|String|Append "Attack/Is Attack Blocked?/Guard Total is: " (Utilities|String|ToString(Float) _output_get) " Accuracy Total: " (Utilities|String|ToString(Float) (+ Roll (LocalVariables|GetAccuracy%20Total) (Variables|Default|GetAccuracy)))))
  (if (< _output_get (+ Roll (LocalVariables|GetAccuracy%20Total) (Variables|Default|GetAccuracy)))
    (Development|PrintString 0 "Attack/Is Attack Blocked/ Attack was not blocked")
    (return false)
    (else
      (Development|PrintString 0 "Attack/Is Attack Blocked/ Attack was blocked")
      (return true))))

(fn IsAttackDodged?
  (params (Attacker :type Page%20Object%20Reference) (Target :type Page%20Object%20Reference) (UseDominant :type Boolean) (Roll :type Float%20%28single-precision%29))
  (bind _stats (Variables|/Game/Dojo/Page.Page_C|GetStats Target))
  (bind _inventory (Variables|/Game/Dojo/Page.Page_C|GetInventory Attacker))
  (bind _dexterity (Variables|/Game/Dojo/CharacterStats.CharacterStats_C|GetDexterity _stats))
  (if UseDominant
    (LocalVariables|SetLocal%20Accuracy (Variables|/Game/Dojo/Items/WeaponObject.WeaponObject_C|GetAccuracy (Variables|/Game/Dojo/Items/Inventory.Inventory_C|GetDominant%20Hand _inventory)))
    (else
      (LocalVariables|SetLocal%20Accuracy (Variables|/Game/Dojo/Items/WeaponObject.WeaponObject_C|GetAccuracy (Variables|/Game/Dojo/Items/Inventory.Inventory_C|GetOffHand _inventory)))))
  (Development|PrintString 0 (Utilities|String|Append "Attack/Does Attack HIt/ Die Roll: " (Utilities|String|ToString(Float) Roll) "Accuracy from attack" (Utilities|String|ToString(Float) (Variables|Default|GetAccuracy)) " Accuracy From weapon" "Enemies Dexterity" (Utilities|String|ToString(Float) _dexterity)))
  (if (> (+ Roll (+ (LocalVariables|GetLocal%20Accuracy) (Variables|Default|GetAccuracy))) (+ _dexterity 1e+01))
    (return false)
    (else
      (Development|PrintString 0 "Attack/Does Attack Hit/Attack misses the target completely")
      (return true))))

(fn IsHitCritical?
  (params (Attacker :type Page%20Object%20Reference) (Target :type Page%20Object%20Reference) (IsDominant :type Boolean) (Roll :type Float%20%28single-precision%29))
  (bind _inventory (Variables|/Game/Dojo/Page.Page_C|GetInventory Attacker))
  (bind _total_coverage1 (Default|GetDefensiveStats (Variables|/Game/Dojo/Page.Page_C|GetInventory Target)))
  (if IsDominant
    (LocalVariables|SetLocal%20Accuracy (Variables|/Game/Dojo/Items/WeaponObject.WeaponObject_C|GetAccuracy (Variables|/Game/Dojo/Items/Inventory.Inventory_C|GetDominant%20Hand _inventory)))
    (else
      (LocalVariables|SetLocal%20Accuracy (Variables|/Game/Dojo/Items/WeaponObject.WeaponObject_C|GetAccuracy (Variables|/Game/Dojo/Items/Inventory.Inventory_C|GetOffHand _inventory)))))
  (if (< _total_coverage1 (+ Roll (+ (LocalVariables|GetLocal%20Accuracy) (Variables|Default|GetAccuracy))))
    (Development|PrintString 0 "Attack/IsHitCiritcal/Attack is an excellent hit!")
    (return true)
    (else
      (Development|PrintString 0 "Attack/IsHitCiritcal/Attack is just a regular hit")
      (return false))))

(fn GetDeflectionModifier
  (params (Attacker :type Page%20Object%20Reference) (Target :type Page%20Object%20Reference) (IsDominant :type Boolean) (Roll :type Float%20%28single-precision%29))
  (bind _inventory (Variables|/Game/Dojo/Page.Page_C|GetInventory Attacker))
  (bind _dominant_hand (Variables|/Game/Dojo/Items/Inventory.Inventory_C|GetDominant%20Hand _inventory))
  (bind _offhand (Variables|/Game/Dojo/Items/Inventory.Inventory_C|GetOffHand _inventory))
  (bind _total_deflection1 (Default|GetDefensiveStats (Variables|/Game/Dojo/Page.Page_C|GetInventory Target)))
  (LocalVariables|SetLocal%20Deflection _total_deflection1)
  (if IsDominant
    (LocalVariables|SetLocal%20Accuracy (+ (Variables|/Game/Dojo/Items/WeaponObject.WeaponObject_C|GetAccuracy _dominant_hand) (Variables|/Game/Dojo/Items/WeaponObject.WeaponObject_C|GetContact _dominant_hand)))
    (else
      (LocalVariables|SetLocal%20Accuracy (+ (Variables|/Game/Dojo/Items/WeaponObject.WeaponObject_C|GetAccuracy _offhand) (Variables|/Game/Dojo/Items/WeaponObject.WeaponObject_C|GetContact _offhand)))))
  (return (/ (- (+ Roll (+ (LocalVariables|GetLocal%20Accuracy) (Variables|Default|GetAccuracy))) (LocalVariables|GetLocal%20Deflection)) (+ Roll (+ (LocalVariables|GetLocal%20Accuracy) (Variables|Default|GetAccuracy))))))