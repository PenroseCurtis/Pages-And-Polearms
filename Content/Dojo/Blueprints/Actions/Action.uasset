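; Action is a base-looking Blueprint for dojo actions, with Click, Hover and GetAttacks functions that all have empty bodies.
; GetAttacks holds disconnected leftover logic that never runs.
; That logic would build an action list from a Page's spells, special attacks, current stance attacks and enchantment attacks, printing a warning when no stance is selected.
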(fn Click)

(fn Hover
  (params (Parent :type Action%20Button%20Object%20Reference)))

(fn GetAttacks
  (params (Page :type Page%20Object%20Reference)))