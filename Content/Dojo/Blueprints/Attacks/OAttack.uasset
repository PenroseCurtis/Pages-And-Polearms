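; OAttack is an attack object that manages and validates targets for a Page attacker in a tile-based game.
; Targets are added up to a maximum, then Attack filters them by allowed class, tile range and a self-targeting flag.
; If enough remain, Attack clears the attacker's PendingAttack and returns true, though the attack itself is only a debug print.
; TriggerConditionMet always returns true.
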(fn GetValidTargets
  (params (Targets :type Array%20of%20Object%20Object%20References) (Attacker :type Page%20Object%20Reference))
  (Utilities|Array|Clear (LocalVariables|GetLocal%20targets))
  (for _array_element Targets
    (bind _valid (CallFunction|IsTargetValid _array_element Attacker))
    (if _valid
      (Utilities|Array|Add (LocalVariables|GetLocal%20targets) _array_element)))
  (return (LocalVariables|GetLocal%20targets)))

(fn Attack
  (params (Attacker :type Page%20Object%20Reference))
  (bind _local_targets1 (CallFunction|GetValidTargets (Variables|Default|GetTargetList) Attacker))
  (Variables|Default|SetTargetList _local_targets1)
  (bind _returnvalue (CallFunction|DoIHaveEnoughTargets))
  (if _returnvalue
    (Development|PrintString 0 "Attack!")
    (Variables|/Game/Dojo/Page.Page_C|SetpendingAttack Attacker 0)
    (return true)
    (else
      (Development|PrintString 0 "Not enough Targets")
      (return false))))

(fn IsTargetValid
  (params (Target :type Object%20Object%20Reference) (Page%20attacking :type Page%20Object%20Reference))
  (bind _valid (CallFunction|IsTargetofCorrectType Target))
  (bind _witihin_range (CallFunction|IsTargetWithinRange Page%20attacking Target))
  (bind _yes_no (CallFunction|IsAttackerTarget Target Page%20attacking))
  (return (Math|Boolean|ANDBoolean _valid _witihin_range (or (not _yes_no) (Variables|Default|GetSelf%20Targettable)))))

(fn IsTargetofCorrectType
  (params (Target :type Object%20Object%20Reference))
  (for _array_element (Variables|Default|GetTargetTypes)
    (if (Utilities|ClassIsChildOf (Utilities|GetClass Target) _array_element)
      (LocalVariables|SetisValid true)))
  (return (LocalVariables|GetisValid)))

(fn IsTargetWithinRange
  (params (Attacker :type Page%20Object%20Reference) (Target :type Object%20Object%20Reference))
  (bind _newparam (Class|WorldObject|GetLocation(Message) Target))
  (bind _distance (Class|WorldObject|GetDistancefromTile(Message) Attacker _newparam))
  (return (<= _distance (Variables|Default|GetRange))))

(fn Addtargets
  (params (Targets :type Array%20of%20Object%20Object%20References))
  (for _array_element Targets
    (if (< (Utilities|Array|Length (Variables|Default|GetTargetList)) (Variables|Default|GetMax%20Targets))
      (Math|Integer|IncrementInt (LocalVariables|GetnumbTargetsAdded)
        (:%20%20
          (Utilities|Array|Add (LocalVariables|GettargetsAdded) _array_element)
          (Utilities|Array|Add (Variables|Default|GetTargetList) _array_element)))))
  (return (LocalVariables|GetnumbTargetsAdded) (LocalVariables|GettargetsAdded)))

(fn IsAttackerTarget
  (params (Target :type Object%20Object%20Reference) (Attacker :type Page%20Object%20Reference))
  (return (== Target Attacker)))

(fn DoIHaveEnoughTargets
  (return (>= (Utilities|Array|Length (Variables|Default|GetTargetList)) (Variables|Default|GetMin%20Targets))))

(fn TriggerConditionMet?
  (return true))