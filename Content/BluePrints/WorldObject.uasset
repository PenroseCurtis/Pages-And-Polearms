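; WorldObject is a Blueprint interface, judging by its empty stubs, that gives objects in the game world a common set of calls.
; Action functions cover overlap, teleporting, path movement, status effects, damage to vitality, stamina and mana, and showing attack UI.
; Query functions expose name, location, tile distance, off-turn actions, opacity, weight and type, pointing to turn-based, tile-based play.
; It holds no logic, only placeholder return values.
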(fn OnOverLap)

(fn GetName
  (return ""))

(fn GetLocation
  (return 0))

(fn Teleport
  (params (Steps :type Array%20of%20BP%20Tile%20Object%20References)))

(fn ApplyStatus
  (params (Status%20Effects :type Array%20of%20O%20Status%20Object%20References)))

(fn Damage
  (params (Vitality :type Array%20of%20Floats%20%28single-precision%29) (Stamina :type Array%20of%20Floats%20%28single-precision%29) (Mana :type Array%20of%20Floats%20%28single-precision%29)))

(fn MoveTarget
  (params (Path :type Array%20of%20BP%20Tile%20Object%20References)))

(fn GetDistancefromTile
  (params (Tile :type BP%20Tile%20Object%20Reference))
  (return 0))

(fn ShowAttacksUI
  (params (Attacks :type Array%20of%20Strings)))

(fn GetOffTurnActions
  (return 0))

(fn GetOpacity
  (return 0.0))

(fn GetWeight
  (return 0.0))

(fn GetType
  (return "NewEnumerator0"))